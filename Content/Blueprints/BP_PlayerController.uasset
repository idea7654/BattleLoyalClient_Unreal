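; BP_PlayerController is a player controller that drives the start-position selection screen shown before play begins.
; OtherUserSetPos increments a counter for the chosen one of three sectors and writes it to the WBP_StartPos widget as a Korean headcount label.
; StartSign removes that widget, switches input to game-only and hides the mouse cursor.
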(event `self.StartSign`
  (`Widget.RemoveFromParent` (`self.StartPosWidget`))
  (`WidgetBlueprintLibrary.SetInputMode_GameOnly` (`GameplayStatics.GetPlayerController` 0))
  (set `self.bShowMouseCursor` false))

(event `self.OtherUserSetPos`
  (params (Sector :type Integer))
  (bind _aswbp_start_pos (cast `/Game/UI/WBP_StartPos` (`self.StartPosWidget`)))
  (switch `int` Sector
    (:`1`
      (bind _output_get (set `self.Section1Count` (+ (`self.Section1Count`) 1)))
      (set `/Game/UI/WBP_StartPos.Section1` (`KismetStringLibrary.Concat_StrStr` (`KismetStringLibrary.Conv_IntToString` _output_get) "명") _aswbp_start_pos))
    (:`2`
      (bind _output_get_2 (set `self.Section2Count` (+ (`self.Section2Count`) 1)))
      (set `/Game/UI/WBP_StartPos.Section2` (`KismetStringLibrary.Concat_StrStr` (`KismetStringLibrary.Conv_IntToString` _output_get_2) "명") _aswbp_start_pos))
    (:`3`
      (bind _output_get_3 (set `self.Section3Count` (+ (`self.Section3Count`) 1)))
      (set `/Game/UI/WBP_StartPos.Section3` (`KismetStringLibrary.Concat_StrStr` (`KismetStringLibrary.Conv_IntToString` _output_get_3) "명") _aswbp_start_pos))))

(fn `UserConstructionScript`)